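; Brimstone orb effect area that applies a hazard debuff to characters inside its sphere.
; The first actor overlap debuffs that actor and starts a looping timer.
; Each tick reapplies the debuff to every overlapping ConanCharacter and clears the timer once none remain.
; Debuffs go through each target's BuffSystemInterface component, passing potency and crediting the instigator as damage causer.
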(event `self.ReceiveActorBeginOverlap`
  (params (OtherActor :type "Actor Object Reference"))
  ;[1 1 1] An Actor enters area, start doing damage
  (if (not (`KismetSystemLibrary.K2_TimerExistsHandle` (`self.Timer Handle`)))
    (bind _returnvalue (`KismetSystemLibrary.K2_SetTimerDelegate` (delegate `Do Gas Orb Buff`) (`self.Debuff Frequency`) true))
    (set `self.Timer Handle` _returnvalue)
    (`self.Apply Debuff` OtherActor)))

(event `Do Gas Orb Buff`
  (bind _overlappingactors (`PrimitiveComponent.GetOverlappingActors` (`self.Sphere`) "/Script/ConanSandbox.ConanCharacter"))
  ;[1 1 1] Check and apply damage to actors within sphere radious
  (if (> (`KismetArrayLibrary.Array_Length` _overlappingactors) 0)
    (for _array_element _overlappingactors
      (`self.Apply Debuff` _array_element))
    (else
      (`KismetSystemLibrary.K2_ClearAndInvalidateTimerHandle` (`self.Timer Handle`)))))

(fn `Apply Debuff`
  (params (Target :type "Actor Object Reference"))
  (bind _returnvalue (`self.GetComponentByInterface` Target "/Game/Systems/Buffs/BuffSystemInterface.BuffSystemInterface_C"))
  (bind _instigator (`self.Instigator`))
  ;[1 1 1] Check if target is valid and apply proper debuff
  (`/Engine/EditorBlueprintResources/StandardMacros.IsValid` _returnvalue
    (:`Is Valid`
      (message `/Game/Systems/Buffs/BuffSystemInterface.AddBuffCall` _returnvalue (`self.Hazard Debuff`) _instigator (`self.Potency`) (`Pawn.GetController` _instigator)))))

(fn `UserConstructionScript`
  (`parent.UserConstructionScript`))