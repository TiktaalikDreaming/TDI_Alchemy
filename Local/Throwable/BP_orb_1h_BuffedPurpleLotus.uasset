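; One-handed Buffed Purple Lotus throwable orb, a child Blueprint that adds cosmetic orientation for its Grease component.
; On BeginPlay, outside dedicated servers, it sets Grease to absolute rotation and plays the Update_liquid_rot timeline.
; Each timeline update turns Grease to player character 0's forward vector, independent of the orb's own rotation.
; All other behavior comes from the parent class, whose BeginPlay runs afterward.
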(event `self.ReceiveBeginPlay`
  (`|ExecutionSequence`
    (:`then_0`
      (if (not (`KismetSystemLibrary.IsDedicatedServer`))
        (set `SceneComponent.bAbsoluteRotation` true (`self.grease`))
        (`Timeline|update_liquid_rot`
          (:`Update`
            (`SceneComponent.K2_SetWorldRotation` (`self.grease`) (`KismetMathLibrary.MakeRotFromX` (`self.GetActorForwardVector` (`GameplayStatics.GetPlayerCharacter` 0))) false false)))))
    (:`then_1`
      (`parent.ReceiveBeginPlay`))))

(fn `UserConstructionScript`
  (`parent.UserConstructionScript`))