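; Interactable lore skull for the Dark Library that trades a Fragment of Power for random knowledge items.
; First use grants a starter item and force-learns the access feat.
; Later uses build candidates from DT_Darklibrary, mapping items to feats via ItemTable's light/heavy health damage fields.
; It removes carried or learned entries, grants a random remainder and deletes a fragment from the backpack only, even when found on the shortcut bar.
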(event `InteractableInterface.InteractableActivate`
  (params (Component :type "PrimitiveComponent Object Reference") (Instigator :type "PlayerController Object Reference") (HitIndex :type Integer) (TriggeredFromRadialWheel :type Boolean))
  (bind _conancharacterref (`self.ConanCharacterRef`))
  (bind _conancharacterref_2 (`self.ConanCharacterRef`))
  (bind _localdarklibraryitems (`self.LocalDarkLibraryItems`))
  (bind _localdarklibraryitems_2 (`self.LocalDarkLibraryItems`))
  (bind _conancharacterref_3 (`self.ConanCharacterRef`))
  (bind _returnvalue (`KismetArrayLibrary.Array_Length` (`self.LocalDarkLibraryItems`)))
  (bind _returnvalue_2 (`ItemInventory.GetInventoryByType` (`self.ConanCharacterRef`) "Backpack"))
  (`KismetSystemLibrary.PrintString` "Clicked")
  (bind _asconan_character (cast `ConanCharacter` (`Controller.K2_GetPawn` Instigator))
    (:`then`
      (set `self.ConanCharacterRef` _asconan_character)
      (bind _returnvalue_3 (`ConanCharacter.GetProgressionSystem` _conancharacterref))
      (bind _asbase_player_char_interface (cast `/Game/Systems/Interfaces/BasePlayerCharInterface` _conancharacterref))
      (`/Game/Systems/Interfaces/BasePlayerCharInterface.AddJourneyEventInterfaceCall` _asbase_player_char_interface "EsotericLibrary")
      (if (`ProgressionSystem.IsFeatPurchased` _returnvalue_3 15000)
        (`KismetSystemLibrary.PrintString` "Not First Time")
        (if (`ItemInventory.HasItemByTemplateID` (`ItemInventory.GetInventoryByType` (`self.ConanCharacterRef`) "Backpack") 11103 1)
          (set `self.LocalActiveInventory` null)
          ;[1 1 1] 1 - Store all library items in an array
          (bind _outrownames (`DataTableFunctionLibrary.GetDataTableRowNames` "/Game/Items/LoreObjects/DT_Darklibrary.DT_Darklibrary" :!label _label))
          (for _array_element _outrownames
            (bind _returnvalue_4 (`|GetDataTableRow` "/Game/Items/LoreObjects/DT_Darklibrary.DT_Darklibrary" _array_element)
              (:`then`
                (`KismetArrayLibrary.Array_AddUnique` (`self.LocalDarkLibraryItems`) (break `/Game/Items/LoreObjects/DarkLibrary` _returnvalue_4)))))
          ;[1 1 1] 2 - Store all items and feats in a map
          (for _array_element_2 _
            (bind _returnvalue_5 (`|GetDataTableRow` "/Game/Items/ItemTable.ItemTable" (`KismetStringLibrary.Conv_StringToName` (`KismetStringLibrary.Conv_IntToString` _array_element_2)))
              (:`then`
                (bind ((`DamageHealthLight_OnHit` _damagehealthlight_onhit) (`DamageHealthHeavy_OnHit` _damagehealthheavy_onhit)) (break `ItemTableRow` _returnvalue_5))
                (if (!= _damagehealthlight_onhit 15000)
                  (`BlueprintMapLibrary.Map_Add` (`self.ItemToFeatMap`) _array_element_2 _damagehealthlight_onhit)
                  (elif (!= _damagehealthheavy_onhit 15000)
                    (`BlueprintMapLibrary.Map_Add` (`self.ItemToFeatMap`) _array_element_2 _damagehealthheavy_onhit))))))
          ;[1 1 1] 3 - Remove any potential handout items that players already have in their inventory
          (bind (_arrayindex _arrayelement) (`/Engine/EditorBlueprintResources/StandardMacros.ReverseForEachLoop` (`self.LocalDarkLibraryItems`))
            (:`LoopBody`
              (if (or (`ItemInventory.HasItemByTemplateID` (`ItemInventory.GetInventoryByType` _conancharacterref_3 "Backpack") _arrayelement 1) (`ItemInventory.HasItemByTemplateID` (`ItemInventory.GetInventoryByType` _conancharacterref_3 "ShortcutBar") _arrayelement 1))
                (`KismetArrayLibrary.Array_Remove` (`self.LocalDarkLibraryItems`) _arrayindex)))
            (:`Completed`
              ;[1 1 1] 4 - Remove any items that players have the feats for
              (bind _returnvalue_6 (`ConanCharacter.GetProgressionSystem` (`self.ConanCharacterRef`)))
              (bind (_arrayindex_2 _arrayelement_2) (`/Engine/EditorBlueprintResources/StandardMacros.ReverseForEachLoop` _localdarklibraryitems_2)
                (:`LoopBody`
                  (bind (_value _returnvalue_7) (`BlueprintMapLibrary.Map_Find` (`self.ItemToFeatMap`) _arrayelement_2))
                  (if (and _returnvalue_7 (`ProgressionSystem.IsFeatPurchased` _returnvalue_6 _value))
                    (`KismetArrayLibrary.Array_Remove` _localdarklibraryitems_2 _arrayindex_2)))
                (:`Completed`
                  (if (> _returnvalue 0)
                    (if (== _returnvalue 1)
                      (`ConanCharacter.ClientHUDShowNotification` (`self.ConanCharacterRef`) (`self.AllKnowledgeLearned`) false true))
                    (`ItemInventory.AddItemTemplate` _returnvalue_2 (`KismetArrayLibrary.Array_Get` _localdarklibraryitems (`KismetMathLibrary.RandomIntegerInRange` 0 (- (`KismetArrayLibrary.Array_Length` _localdarklibraryitems) 1))) (`ItemInventory.GetFirstFreeIndex` _returnvalue_2 false) "loot_environment" 1 true 100.0 100.0) ; To Spawn an item with 0 - 100% durability, modify the Durability Percentage parameter and leave the Durability parameter to its default -1 value. To set a specific Durability value, change the Durability parameter from 0 - MaxDurability. (Values are caped)
                    (`ConanCharacter.ClientHUDShowNotification` (`self.ConanCharacterRef`) (`self.DarkLibraryItemGranted`) false true)
                    (`ItemInventory.DeleteItemsByTemplate` _returnvalue_2 11103 "consumed" 1)
                    (else
                      (`ConanCharacter.ClientHUDShowNotification` (`self.ConanCharacterRef`) (`self.AllKnowledgeLearned`) false true)))))))
          (elif (`ItemInventory.HasItemByTemplateID` (`ItemInventory.GetInventoryByType` (`self.ConanCharacterRef`) "ShortcutBar") 11103 1)
            (set `self.LocalActiveInventory` null)
            (goto _label)
            (else
              (`ConanCharacter.ClientHUDShowNotification` (`self.ConanCharacterRef`) (`self.NeedFragmentOfPower`) false true))))
        (else
          ;[1 1 1] First Time useage
          (`KismetSystemLibrary.PrintString` "First Time")
          (bind _returnvalue_8 (`ConanCharacter.GetBackpackInventory` (`self.ConanCharacterRef`)))
          (`ItemInventory.AddItemTemplate` _returnvalue_8 30000 -1 "loot_environment" 1 false 100.0 -1.0) ; To Spawn an item with 0 - 100% durability, modify the Durability Percentage parameter and leave the Durability parameter to its default -1 value. To set a specific Durability value, change the Durability parameter from 0 - MaxDurability. (Values are caped)
          (`ConanCharacter.ClientHUDShowNotification` _conancharacterref_2 (`self.DarkLibraryAccessed`) false true)
          (bind _returnvalue_9 (`ConanCharacter.GetProgressionSystem` _conancharacterref_2))
          (`ProgressionSystem.ServerForceLearnFeat` _returnvalue_9 15000 true false))))
    (:`CastFailed`
      (`KismetSystemLibrary.PrintString` "AWOOGA"))))

(fn `UserConstructionScript`
  (`parent.UserConstructionScript`))