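; Radium variant of a corruption buff component that keeps the affected character corrupted and modifies the damage of non-player characters.
; On start it caches the owner's energy receiver, then each tick raises corruption energy to a target amount if below it, without lowering higher values.
; For non-players, ticks also apply multiplicative melee and ranged damage modifiers, which clearing neutralizes by re-adding them at one.
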(event `self.StartBuff`
  (params (BuffPotency :type Integer) (OwningCharacter :type "ConanCharacter Object Reference") (Instigator :type "Controller Object Reference"))
  (`parent.StartBuff` BuffPotency OwningCharacter Instigator)
  (set `self.EnergyReceiverComponent` (`Actor.GetComponentByClass` (`self.OwningCharacter`) "/Script/ConanSandbox.EnergyReceiverComponent")))

(event `self.GameplayEffectToApplyOnBuffTick`
  (bind _owningcharacter (`self.OwningCharacter`))
  (bind _energyreceivercomponent (`self.EnergyReceiverComponent`))
  (`parent.GameplayEffectToApplyOnBuffTick`)
  (`/Engine/EditorBlueprintResources/StandardMacros.IsValid` _energyreceivercomponent
    (:`Is Valid`
      (if (< (`EnergyReceiverComponent.GetEnergy` _energyreceivercomponent "EnergyType_Corruption") (`self.NewCorruptionAmount`))
        (`EnergyReceiverComponent.SetEnergy` _energyreceivercomponent "EnergyType_Corruption" (`self.NewCorruptionAmount`) 0.0)))
    (:`Is Not Valid`
      _))
  (if (not (`ConanCharacter.IsPlayer` _owningcharacter))
    (`ConanCharacter.AddFloatStatModifier` _owningcharacter "DamageModifierMelee" "Buff" "Multiply" 0.0 "Replace")
    (`ConanCharacter.AddFloatStatModifier` _owningcharacter "DamageModifierRanged" "Buff" "Multiply" 0.0 "Replace")))

(event `self.GameplayEffectToApplyOnBuffCleared`
  (bind _owningcharacter (`self.OwningCharacter`))
  (`parent.GameplayEffectToApplyOnBuffCleared`)
  (if (not (`ConanCharacter.IsPlayer` _owningcharacter))
    (`ConanCharacter.AddFloatStatModifier` _owningcharacter "DamageModifierMelee" "Buff" "Multiply" 1.0 "Replace")
    (`ConanCharacter.AddFloatStatModifier` _owningcharacter "DamageModifierRanged" "Buff" "Multiply" 1.0 "Replace")))