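; Test one-handed radium torch held item, flagged as a glow stick in its construction script.
; Every Tick, except on dedicated servers, it checks whether the owning character is swimming.
; Swimming shows the Cheren particle effect, hides the regular one and deactivates EnergySourceRadiation; otherwise it reverses all three.
; The logic attaching the green glow light to the tip socket is unreachable.
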(event `self.ReceiveEndPlay`
  (params (EndPlayReason :type "EEndPlayReason Enum" :default "Destroyed")))

(event `self.ReceiveTick`
  (params (DeltaSeconds :type "Float (single-precision)"))
  (bind _cheren (`self.Cheren`))
  (bind _energysourceradiation (`self.EnergySourceRadiation`))
  (bind _particlesystem1 (`self.ParticleSystem1`))
  (if (`KismetSystemLibrary.IsDedicatedServer`)
    _
    (elif (`NavMovementComponent.IsSwimming` (`Character.CharacterMovement` (`self.CharacterOwner`)))
      (`ParticleSystemComponent.SetEmitterEnable` _cheren "One" true)
      (`ParticleSystemComponent.SetEmitterEnable` _cheren "Two" true)
      (`SceneComponent.SetVisibility` _cheren true true)
      (`ParticleSystemComponent.SetEmitterEnable` _particlesystem1 "One" false)
      (`ParticleSystemComponent.SetEmitterEnable` _particlesystem1 "Two" false)
      (`ParticleSystemComponent.SetEmitterEnable` _particlesystem1 "Three" false)
      (`SceneComponent.SetVisibility` _particlesystem1 false true)
      (`ActorComponent.SetActive` _energysourceradiation false false)
      (else
        (`ParticleSystemComponent.SetEmitterEnable` _cheren "One" false)
        (`ParticleSystemComponent.SetEmitterEnable` _cheren "Two" false)
        (`SceneComponent.SetVisibility` _cheren false true)
        (`ParticleSystemComponent.SetEmitterEnable` _particlesystem1 "One" true)
        (`ParticleSystemComponent.SetEmitterEnable` _particlesystem1 "Two" true)
        (`ParticleSystemComponent.SetEmitterEnable` _particlesystem1 "Three" true)
        (`SceneComponent.SetVisibility` _particlesystem1 true true)
        (`ActorComponent.SetActive` _energysourceradiation true false)))))

(fn `UserConstructionScript`
  (set `self.IsGlowStick` true)
  (`parent.UserConstructionScript`))