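; Placeable lotus bowl that shows its inventory contents as a powder mesh filling the bowl.
; Non-dedicated instances create an inventory monitor at BeginPlay; item add, remove and stat-change events refresh the LotusLevel mesh.
; Two timelines act as curve lookups, scrubbed by first-slot stack size, setting height, then scale and visibility.
; A cascade of template ID checks sets the "powder" slot material between those steps.
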(event `self.ReceiveBeginPlay`
  (bind _placeableinventory (`self.PlaceableInventory`))
  (bind _placeableinventory_2 (`self.PlaceableInventory`))
  (bind _placeableinventory_3 (`self.PlaceableInventory`))
  (bind _returnvalue (`KismetMathLibrary.FMin` (/ (`KismetMathLibrary.Conv_IntToDouble` (`GameItem.GetIntStat` (`ItemInventory.GetItem` (`self.PlaceableInventory`) 0) "StackSize")) 100.0) 1.0))
  (`parent.ReceiveBeginPlay`)
  (if (`KismetSystemLibrary.IsDedicatedServer`)
    _
    (else
      _))
  (`|ExecutionSequence`
    (:`then_0`
      ;[0.02499 0.09524 0.16] Make sure the the inventory is loaded even if it hasn't been interacted with.
      (if (not (`KismetSystemLibrary.IsDedicatedServer`))
        (bind _returnvalue_2 (`|GenericCreateObject` "/Script/ConanSandbox.ItemInventoryClientMonitor" self))
        (`ItemInventoryClientMonitor.SetInventory` _returnvalue_2 (`self.PlaceableInventory`))))
    (:`then_1`
      (add `ItemInventory.SignalItemAdded` _placeableinventory_3 (delegate `SetLotusHeight`))
      (add `ItemInventory.SignalItemRemoved` _placeableinventory_3 (delegate `SetLotusHeight`)))
    (:`then_2`
      ;[1 0.6413 0.1882] Set Z location of FoodPlane
      (bind (_direction _height) (`Timeline|Timeline_1` :`NewTime` _returnvalue :!via `SetNewTime` :!label _label)
        (:`Update`
          (`SceneComponent.K2_SetRelativeLocation` (`self.LotusLevel`) (`KismetMathLibrary.MakeVector` 0.0 0.0 _height) false false)
          ;[1 1 1] Set Colour
          (if (> (`ItemInventory.GetResourceCount` _placeableinventory 11125 false) 0)
            (`PrimitiveComponent.SetMaterialByName` (`self.LotusLevel`) "powder" null)
            ;[1 0.6413 0.1882] Set XY scale based on curve to fit the bowl.
            (bind (_direction_2 _scale) (`Timeline|Timeline_0` :`NewTime` _returnvalue :!via `SetNewTime` :!label _label_2)
              (:`Update`
                (`SceneComponent.SetRelativeScale3D` (`self.LotusLevel`) (`KismetMathLibrary.MakeVector` _scale _scale _scale))
                ;[1 0.6413 0.1882] Handle Visibility
                (if (== (`ItemInventory.GetPopulatedItemCount` (`self.PlaceableInventory`) 0 -1) 0)
                  (`SceneComponent.SetVisibility` (`self.LotusLevel`) false false)
                  (else
                    (`SceneComponent.SetVisibility` (`self.LotusLevel`) true false)))))
            (elif (> (`ItemInventory.GetResourceCount` _placeableinventory 11084 false) 0)
              (`PrimitiveComponent.SetMaterialByName` (`self.LotusLevel`) "powder" null)
              (goto _label_2 :!via `SetNewTime`)
              (elif (> (`ItemInventory.GetResourceCount` _placeableinventory 11087 false) 0)
                (`PrimitiveComponent.SetMaterialByName` (`self.LotusLevel`) "powder" null)
                (goto _label_2 :!via `SetNewTime`)
                (elif (> (`ItemInventory.GetResourceCount` _placeableinventory 11122 false) 0)
                  (`PrimitiveComponent.SetMaterialByName` (`self.LotusLevel`) "powder" null)
                  (goto _label_2 :!via `SetNewTime`)
                  (elif (> (`ItemInventory.GetResourceCount` _placeableinventory 11123 false) 0)
                    (`PrimitiveComponent.SetMaterialByName` (`self.LotusLevel`) "powder" null)
                    (goto _label_2 :!via `SetNewTime`)
                    (elif (> (`ItemInventory.GetResourceCount` _placeableinventory_2 2892322 false) 0)
                      (`PrimitiveComponent.SetMaterialByName` (`self.LotusLevel`) "powder" null)
                      (goto _label_2 :!via `SetNewTime`)
                      (elif (> (`ItemInventory.GetResourceCount` _placeableinventory_2 1370395 false) 0)
                        (`PrimitiveComponent.SetMaterialByName` (`self.LotusLevel`) "powder" null)
                        (goto _label_2 :!via `SetNewTime`)
                        (elif (> (`ItemInventory.GetResourceCount` _placeableinventory_2 11121 false) 0)
                          (`PrimitiveComponent.SetMaterialByName` (`self.LotusLevel`) "powder" null)
                          (goto _label_2 :!via `SetNewTime`)
                          (elif (> (`ItemInventory.GetResourceCount` _placeableinventory_2 1370469 false) 0)
                            (`PrimitiveComponent.SetMaterialByName` (`self.LotusLevel`) "powder" null)
                            (goto _label_2 :!via `SetNewTime`)
                            (elif (> (`ItemInventory.GetResourceCount` _placeableinventory_2 2892295 false) 0)
                              (`PrimitiveComponent.SetMaterialByName` (`self.LotusLevel`) "powder" null)
                              (goto _label_2 :!via `SetNewTime`)
                              (elif (> (`ItemInventory.GetResourceCount` _placeableinventory_2 2892317 false) 0)
                                (`PrimitiveComponent.SetMaterialByName` (`self.LotusLevel`) "powder" null)
                                (goto _label_2 :!via `SetNewTime`)
                                (elif (> (`ItemInventory.GetResourceCount` _placeableinventory_2 2892319 false) 0)
                                  (`PrimitiveComponent.SetMaterialByName` (`self.LotusLevel`) "powder" null)
                                  (goto _label_2 :!via `SetNewTime`)
                                  (elif (> (`ItemInventory.GetResourceCount` _placeableinventory_2 2892322 false) 0)
                                    (`PrimitiveComponent.SetMaterialByName` (`self.LotusLevel`) "powder" null)
                                    (goto _label_2 :!via `SetNewTime`)
                                    (elif (> (`ItemInventory.GetResourceCount` _placeableinventory_2 32370531 false) 0)
                                      (`PrimitiveComponent.SetMaterialByName` (`self.LotusLevel`) "powder" null)
                                      (goto _label_2 :!via `SetNewTime`)
                                      (else
                                        (`PrimitiveComponent.SetMaterialByName` (`self.LotusLevel`) "powder" null)
                                        (goto _label_2 :!via `SetNewTime`)))))))))))))))))))))

(event `self.PlaceableInventory.SignalItemIntStatChanged`
  (params (item :type "GameItem Object Reference") (statID :type "EItemIntStatID Enum" :default "MaxStackSize") (statValue :type Integer) (deltaValue :type Integer))
  (goto _label :!via `SetNewTime`))

(event `SetLotusHeight`
  (params (index :type Integer) (item :type "GameItem Object Reference") (dstInventory :type "ItemInventory Object Reference") (dstIndex :type Integer))
  ;[1 0.6413 0.1882] Set Z location of FoodPlane
  (goto _label :!via `SetNewTime`))

(fn `UserConstructionScript`
  (`parent.UserConstructionScript`))