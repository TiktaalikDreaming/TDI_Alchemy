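; One-handed radium torch, a glow-stick item with a green tip light that spreads corruption to nearby characters and its wielder.
; Sphere overlaps track affected characters and send a buff on entry, while Tick also registers and buffs through the instigator's controller.
; HazardTick runs ApplyBuff over the tracked list, stacking the Iron King corruption buff.
; Outside dedicated servers, Tick enables the Cheren particle emitters only while the owner swims.
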(event `self.ReceiveBeginPlay`
  (`parent.ReceiveBeginPlay`)
  (`SceneComponent.K2_AttachToComponent` (`self.Light Green Glow`) null "tip" "KeepRelative" "KeepRelative" "KeepRelative" true))

(event `self.Sphere.OnComponentBeginOverlap`
  (params (OverlappedComponent :type "PrimitiveComponent Object Reference") (OtherActor :type "Actor Object Reference") (OtherComp :type "PrimitiveComponent Object Reference") (OtherBodyIndex :type Integer) (bFromSweep :type Boolean) (SweepResult :type "HitResult Structure (by ref)"))
  (bind _instigator (`self.Instigator`))
  (bind _asconan_character (cast `ConanCharacter` OtherActor))
  (bind _returnvalue (`self.GetComponentByInterface` _asconan_character "/Game/Systems/Buffs/BuffSystemInterface.BuffSystemInterface_C"))
  (`/Engine/EditorBlueprintResources/StandardMacros.IsValid` _returnvalue
    (:`Is Valid`
      (`KismetArrayLibrary.Array_Add` (`self.BuffAffectedChars`) _asconan_character)
      (message `/Game/Systems/Buffs/BuffSystemInterface.AddBuffCall` _returnvalue null _instigator 1 (`/Game/Characters/FuncomFunctionLibrary.GetControllerFromActor` _instigator)))))

(event `self.Sphere.OnComponentEndOverlap`
  (params (OverlappedComponent :type "PrimitiveComponent Object Reference") (OtherActor :type "Actor Object Reference") (OtherComp :type "PrimitiveComponent Object Reference") (OtherBodyIndex :type Integer))
  (bind _asconan_character (cast `ConanCharacter` OtherActor))
  (`KismetArrayLibrary.Array_RemoveItem` (`self.BuffAffectedChars`) _asconan_character))

(event `self.ReceiveTick`
  (params (DeltaSeconds :type "Float (single-precision)"))
  (bind _cheren (`self.Cheren`))
  (bind _instigator (`self.Instigator`))
  (bind _controller (`/Game/Characters/FuncomFunctionLibrary.GetControllerFromActor` (`self.Instigator`)))
  (`|ExecutionSequence`
    (:`then_0`
      (if (`KismetSystemLibrary.IsDedicatedServer`)
        _
        (elif (`NavMovementComponent.IsSwimming` (`Character.CharacterMovement` (`self.CharacterOwner`)))
          (`ParticleSystemComponent.SetEmitterEnable` _cheren "One" true)
          (`ParticleSystemComponent.SetEmitterEnable` _cheren "Two" true)
          (else
            (`ParticleSystemComponent.SetEmitterEnable` _cheren "One" false)
            (`ParticleSystemComponent.SetEmitterEnable` _cheren "Two" false)))))
    (:`then_1`
      (`/Engine/EditorBlueprintResources/StandardMacros.IsValid` _controller
        (:`Is Valid`
          (`KismetArrayLibrary.Array_Add` (`self.BuffAffectedChars`) null)
          (message `/Game/Systems/Buffs/BuffSystemInterface.AddBuffCall` (`self.GetComponentByInterface` _controller "/Game/Systems/Buffs/BuffSystemInterface.BuffSystemInterface_C") null _instigator 1 (`/Game/Characters/FuncomFunctionLibrary.GetControllerFromActor` _instigator)))))))

(event `Hazard Tick`
  (for _ (`self.BuffAffectedChars`)
    (`self.Apply Buff` null)))

(fn `Apply Buff`
  (params (Player :type "Actor Object Reference"))
  (bind _returnvalue (`self.GetComponentByInterface` Player "/Game/Systems/Buffs/BuffSystemInterface.BuffSystemInterface_C"))
  (bind _instigator (`self.Instigator`))
  (`/Engine/EditorBlueprintResources/StandardMacros.IsValid` _returnvalue
    (:`Is Valid`
      (for _ (range 1 (+ (`self.Stacks`) 1))
        (message `/Game/Systems/Buffs/BuffSystemInterface.AddBuffCall` _returnvalue "/Game/Systems/Buffs/NPC/BP_AC_Buff_Corruption_IronKing.BP_AC_Buff_Corruption_IronKing_C" _instigator (`self.Potency`) (`Pawn.GetController` _instigator))))))

(fn `UserConstructionScript`
  (set `self.IsGlowStick` true)
  (`parent.UserConstructionScript`))