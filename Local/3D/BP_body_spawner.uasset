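; Server-side spawner that keeps one heroic treasure coffer at a random spawn point, offset from its root.
; Location and rotation use separate random picks, so they can come from different points.
; Pickup spawns an ambush target at the spawner holding the carried item; destruction reports a treasure action and starts a respawn timer.
; ForceSpawnTreasure skips the wait when no treasure exists, and EndPlay destroys any current treasure.
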(event `/Game/Items/Treasures/I_TreasureSpawnerInterface.ForceSpawnTreasure`
  (if (not (`KismetSystemLibrary.IsValid` (`self.CurrentTreasure`)))
    (`KismetSystemLibrary.K2_ClearAndInvalidateTimerHandle` (`self.RespawnTimer`))
    (`self.SelectSpawnPoint`)))

(event `self.ReceiveBeginPlay`
  ;[1 1 1] On Begin Play
  (if (`KismetSystemLibrary.IsServer`)
    (if (not (`KismetSystemLibrary.IsValid` (`self.CurrentTreasure`)))
      (`self.SelectSpawnPoint`))))

(event `SelectSpawnPoint`
  (bind _returnvalue (`KismetArrayLibrary.Array_Length` (`self.SpawnPoints`)))
  ;[1 1 1] Select Spawn Point and Spawn Actor
  (if (not (`KismetSystemLibrary.IsValid` (`self.CurrentTreasure`)))
    (`KismetSystemLibrary.K2_ClearAndInvalidateTimerHandle` (`self.RespawnTimer`))
    (if (>= _returnvalue 1)
      (bind _returnvalue_2 (`|SpawnActorFromClass` (`self.HeroicActorClass`) (`KismetMathLibrary.MakeTransform` (+ (`SceneComponent.K2_GetComponentLocation` (`self.DefaultSceneRoot`)) (.location (`KismetArrayLibrary.Array_Get` (`self.SpawnPoints`) (`KismetMathLibrary.RandomIntegerInRange` 0 (- _returnvalue 1))))) (.rotation (`KismetArrayLibrary.Array_Get` (`self.SpawnPoints`) (`KismetMathLibrary.RandomIntegerInRange` 0 (- _returnvalue 1))))) "AdjustIfPossibleButAlwaysSpawn" "OverrideRootScale" self))
      (bind _asbp_pl_coffer_treasure_base (cast `/Game/Items/Treasures/Placeables/BP_PL_Coffer_Treasure_Base` _returnvalue_2))
      (bind _output_get (set `self.CurrentTreasure` _asbp_pl_coffer_treasure_base))
      (if (`KismetSystemLibrary.IsValid` _output_get)
        (add `self.OnDestroyed` _output_get (delegate `StartRespawnTimer`))
        (add `/Game/Items/Treasures/Placeables/BP_PL_Coffer_Treasure_Base.Signal_CarryablePickedUp` _output_get (delegate `TreasureTaken`))
        (else
          (`self.SelectSpawnPoint`))))))

(event `TreasureTaken`
  (params (GrantedGameItem :type "GameItem Object Reference"))
  ;[1 1 1] Select Spawn Point and Spawn Actor
  (bind _asbpgame_item_carryable (cast `/Game/Items/Carryables/BPGameItemCarryable` GrantedGameItem))
  (`|SpawnActorFromClass` "/Game/Items/Treasures/BP_TreasureAmbushTarget.BP_TreasureAmbushTarget_C" (`self.GetTransform`) "AlwaysSpawn" "OverrideRootScale" null _asbpgame_item_carryable)
  (clear `/Game/Items/Treasures/Placeables/BP_PL_Coffer_Treasure_Base.Signal_CarryablePickedUp` (`self.CurrentTreasure`)))

(event `StartRespawnTimer` :!signature `self.OnDestroyed`
  (params (DestroyedActor :type "Actor Object Reference"))
  ;[1 1 1] Select Spawn Point and Spawn Actor
  (clear `self.OnDestroyed` DestroyedActor)
  (bind _returnvalue (`KismetSystemLibrary.K2_SetTimerDelegate` (`|CreateDelegate` :!event `SelectSpawnPoint`) (`self.RespawnTime`)))
  (set `self.RespawnTimer` _returnvalue)
  (`ConanTelemetryLibrary.ReportHeroicTreasureAction` (`KismetStringLibrary.Conv_IntToString` (`BuildableBase.TemplateId` (`self.CurrentTreasure`))) "pickup" "spawnpoint")
  (set `self.CurrentTreasure` null))

(event `self.ReceiveEndPlay`
  (params (EndPlayReason :type "EEndPlayReason Enum" :default "Destroyed"))
  (bind _currenttreasure (`self.CurrentTreasure`))
  ;[1 1 1] Clean Up Spawned Treasures on End Play
  (`/Engine/EditorBlueprintResources/StandardMacros.IsValid` _currenttreasure
    (:`Is Valid`
      (clear `self.OnDestroyed` _currenttreasure)
      (`KismetSystemLibrary.K2_ClearAndInvalidateTimerHandle` (`self.RespawnTimer`))
      (`self.K2_DestroyActor` _currenttreasure))))

(fn `ClientGetCraftingGUICenterPanel`
  (params (Instigator :type "PlayerController Object Reference"))
  (returns (ReturnValue :type Name))
  (return "None"))

(fn `ClientGetCraftingGUIRightPanel`
  (params (Instigator :type "PlayerController Object Reference"))
  (returns (ReturnValue :type Name))
  (return "None"))

(fn `GetLoreSoundCue`
  (returns (LoreSound :type "SoundCue Object Reference"))
  (return null))

(fn `InteractableActivateDisabled`
  (params (InteractingCharacter :type "ConanCharacter Object Reference"))
  (returns (ReturnValue :type Boolean))
  (return false))

(fn `InteractableCanBeLooted`
  (params (InteractingCharacter :type "ConanCharacter Object Reference"))
  (returns (ReturnValue :type Boolean))
  (return false))

(fn `InteractableDefaultAction`
  (returns (Name :type Text) (Icon :type "Texture2D Object Reference"))
  (return "" null))

(fn `InteractableGetRepairUIModuleName`
  (returns (ReturnValue :type Name))
  (return "None"))

(fn `InteractableGetSimpleDisplayText`
  (returns (ReturnValue :type Text))
  (return ""))

(fn `InteractableGetUIModuleName`
  (returns (ReturnValue :type Name))
  (return "None"))

(fn `InteractableMenuDisabled`
  (params (InteractingCharacter :type "ConanCharacter Object Reference"))
  (returns (ReturnValue :type Boolean))
  (return false))

(fn `InteractableShouldCommand`
  (returns (ReturnValue :type Boolean))
  (return false))

(fn `UserConstructionScript`
  (locals (L_Mesh :type "StaticMesh Object Reference")))