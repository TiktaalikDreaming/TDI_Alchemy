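; Alchemy mixer crafting station that can explode when an item is crafted or when it takes damage.
; Crafting rolls a rare failure chance, lowered by an artisan thrall's tier; damage rolls against its amount.
; Three stored resource types set the blast's strength, which gates detonation and scales layered radial damage where PvP or a valid placer allows it.
; Detonation also spawns an oil fire, multicasts effects and destroys the bench after a delay.
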(event SignalItemCrafted(CraftingQueue)
  (params (recipeItem :type Recipe%20Item%20Object%20Reference) (gameItem :type Game%20Item%20Object%20Reference) (stackSize :type Integer))
  (bind _returnvalue (Math|Random|RandomInteger 500))
  (bind _returnvalue_2 (Math|Random|RandomInteger 500))
  (bind _returnvalue_3 (Math|Random|RandomInteger 500))
  (bind _explosionorigin (Variables|Default|GetExplosionOrigin))
  (bind _placeableinventory (Variables|Default|GetPlaceableInventory))
  (bind _returnvalue_4 (Transformation|GetWorldLocation _explosionorigin))
  (bind _returnvalue_5 (Class|ItemInventory|GetResourceCount _placeableinventory 22120002 false))
  (bind _returnvalue_6 (Class|ItemInventory|GetResourceCount _placeableinventory 14183 false))
  (bind _returnvalue_7 (Class|ItemInventory|GetResourceCount _placeableinventory 22120004 false))
  (bind _returnvalue_8 (+ _returnvalue_3 _returnvalue_2 _returnvalue))
  (bind _returnvalue_9 (/ _returnvalue_5 6))
  (bind _returnvalue_10 (/ _returnvalue_7 2))
  (bind _returnvalue_11 (* _returnvalue_6 4))
  (bind _returnvalue_12 (+ _returnvalue_9 _returnvalue_11 _returnvalue_10))
  (bind _returnvalue_13 (Math|Conversions|ToFloat(Integer) _returnvalue_12))
  (bind _returnvalue_14 (* _returnvalue_12 9))
  (bind _returnvalue_15 (Math|Float|Power _returnvalue_13 0.333333333333))
  (bind _returnvalue_16 (* _returnvalue_15 4.5e+02))
  (bind _returnvalue_17 (* _returnvalue_16 2.0))
  (bind _returnvalue_18 (/ _returnvalue_17 4.0))
  (bind _asthrall_item (Utilities|Casting|CastToThrallItem (Class|ItemInventory|GetFirstItemAvailable (Class|ItemInventory|GetInventorybyType (Variables|Default|GetPlaceableInventory) 0 "CraftingArtisanInventory")))
    (:then
      (Math|Integer|CompareInt _returnvalue_8 (- 68 (* (Class|GameItem|GetIntStat _asthrall_item "CrafterTier") 16))
        (:<
          _)))
    (:CastFailed
      (Math|Integer|CompareInt _returnvalue_8 68
        (:<
          _))))
  (Class|GameEventDBLibrary|LogGameEventBuildableDemolished self 0 0 false)
  (Math|Integer|CompareInt _returnvalue_12 20
    (:>
      (if (not (Variables|Default|GetHasBlownUp))
        (Class|PersistenceComponent|SetDirty (Variables|Default|GetConanBuildingPersistence) true 1.0)
        (CallFunction|CleanUpComponents)
        (Utilities|FlowControl|Delay (Math|Random|RandomFloatinRange 0.2 0.5))
        (bind _asconan_game_state (Utilities|Casting|CastToConanGameState (Game|GetGameState)))
        (if (or (Class|ConanGameState|IsPVPAllowed _asconan_game_state) (Utilities|IsValid (CallFunction|GetInstigatorOfPlacement)))
          ;[1 1 1] Do not damage Resource actors, otherwise explosion could cause a fracturation of their destructible meshes
          (if (Networking|IsDedicatedServer)
            (Utilities|Array|Clear (Variables|Default|GetIgnoreActors))
            (else
              (bind _outactors (Actor|GetAllActorsOfClass "/Game/Systems/Survival/Gathering/BP_ResourceActor.BP_ResourceActor_C"))
              (bind _output_get (Variables|Default|SetIgnoreActors _outactors))))
          (Utilities|Array|Add _output_get self)
          (|ApplyRadialDamagewithFalloffAsync (Math|Conversions|ToFloat(Integer) (/ _returnvalue_14 3)) 0.0 _returnvalue_4 (/ _returnvalue_16 3.0) _returnvalue_16 3.0 "/Game/Systems/Progression/DmgTypeHealth_BP.DmgTypeHealth_BP_C" 0 self (CallFunction|GetInstigatorOfPlacement) "ECC_GameTraceChannel17"
            (:then
              (|ApplyRadialDamagewithFalloffAsync (Math|Conversions|ToFloat(Integer) _returnvalue_14) 1.0 _returnvalue_4 _returnvalue_18 _returnvalue_17 3.0 "/Game/Systems/Progression/DmgTypeHealth_BP.DmgTypeHealth_BP_C" 0 self (CallFunction|GetInstigatorOfPlacement) "ECC_Visibility"
                (:then
                  (|ApplyRadialDamagewithFalloffAsync (Math|Conversions|ToFloat(Integer) (* _returnvalue_14 12)) 0.0 _returnvalue_4 _returnvalue_18 _returnvalue_17 3.0 "/Game/Systems/Combat/Dmg_Explosive.Dmg_Explosive_C" 0 self (CallFunction|GetInstigatorOfPlacement) "ECC_Visibility"
                    (:then
                      _)))))))
        (bind _returnvalue_19 (Game|SpawnActorfromClass "/Game/Items/Explosives/BP_Oil_Fire_Large.BP_Oil_Fire_Large_C" (Transformation|GetWorldTransform (Variables|Default|GetExclusivePlacementSphere)) "AlwaysSpawn" self (Pawn|GetControlledPawn (CallFunction|GetInstigatorOfPlacement))))
        (Variables|/Game/Items/Weapons/Orbs/BP_Orb_Effect_Master.BP_Orb_Effect_Master_C|SetShouldBePlayerDamage _returnvalue_19 true)
        (CallFunction|MulticastExplosion)
        (Utilities|FlowControl|Delay 3e+01)
        (Actor|DestroyActor)
        (Class|GameEventDBLibrary|LogGameEventBuildableDemolished self 0 0 true)))))

(event OnComponentHit(StaticMesh)
  (params (HitComponent :type Primitive%20Component%20Object%20Reference) (OtherActor :type Actor%20Object%20Reference) (OtherComp :type Primitive%20Component%20Object%20Reference) (NormalImpulse :type Vector) (Hit :type Hit%20Result%20Structure%20%28by%20ref%29))
  ;[1 1 1] Bump Fuse Start
)

(event Custom|CleanUpComponents
  (bind _skeletalmesh (Variables|Default|GetSkeletalMesh))
  (bind _placementcheckbox (Variables|Default|GetPlacementCheckBox))
  (bind _checkcornersbox (Variables|Default|GetCheckCornersBox))
  (bind _checkforcontactbox (Variables|Default|GetCheckForContactBox))
  (bind _exclusiveplacementsphere (Variables|Default|GetExclusivePlacementSphere))
  (bind _overlappingbuildingblockerboxcheck (Variables|Default|GetOverlappingBuildingBlockerBoxCheck))
  (bind _directionindicatormesh (Variables|Default|GetDirectionIndicatorMesh))
  ;[1 1 1] Clean Up Components
  (if (not (Variables|Default|GetCleanupDone))
    (Utilities|FlowControl|Sequence
      (:then_1
        (Utilities|IsValid _placementcheckbox
          (:Is%20Valid
            (Components|DestroyComponent _placementcheckbox))))
      (:then_2
        (Utilities|IsValid _checkcornersbox
          (:Is%20Valid
            (Components|DestroyComponent _checkcornersbox))))
      (:then_3
        (Utilities|IsValid _checkforcontactbox
          (:Is%20Valid
            (Components|DestroyComponent _checkforcontactbox))))
      (:then_4
        (Utilities|IsValid _skeletalmesh
          (:Is%20Valid
            (Components|DestroyComponent _skeletalmesh))))
      (:then_5
        (Utilities|IsValid _exclusiveplacementsphere
          (:Is%20Valid
            (Components|DestroyComponent _exclusiveplacementsphere))))
      (:then_6
        (Utilities|IsValid _overlappingbuildingblockerboxcheck
          (:Is%20Valid
            (Components|DestroyComponent _overlappingbuildingblockerboxcheck))))
      (:then_7
        (Utilities|IsValid _directionindicatormesh
          (:Is%20Valid
            (Components|DestroyComponent _directionindicatormesh))))
      (:then_8
        (Variables|Default|SetCleanupDone true)))))

(event Custom|MulticastExplosion
  (bind _returnvalue (Math|Random|RandomFloatinRange 0.75 3.0))
  (bind _staticmesh (Variables|Default|GetStaticMesh))
  (bind _staticmesh_2 (Variables|Default|GetStaticMesh))
  (bind _returnvalue_2 (Transformation|GetWorldLocation _staticmesh))
  ;[1 1 1] Explosion
  (Rendering|SetVisibility _staticmesh_2 false false)
  (Utilities|FlowControl|Sequence
    (:then_0
      (Collision|SetCollisionEnabled _staticmesh_2 "NoCollision"))
    (:then_1
      (Collision|SetCollisionEnabled (Variables|Default|GetDestructible) "NoCollision"))
    (:then_2
      (Rendering|SetVisibility (Variables|Default|GetExplosion) true false :!label _label)
      (Rendering|SetVisibility (Variables|Default|GetStaticMesh) false false)
      (Class|DreamworldBlueprints|PlaySoundatLocation "/Game/Sound/SFX/Explosions/explosion_large_debris_Cue.explosion_large_debris_Cue" _returnvalue_2)
      (Camera|PlayWorldCameraShake "/Game/Items/Explosives/CameraShake_Explosion.CameraShake_Explosion_C" _returnvalue_2 0.0 3072.0 1.0 true)
      (Class|DestructibleComponent|ApplyRadiusDamage (Variables|Default|GetDestructible) 5e+04 (Transformation|GetWorldLocation (Variables|Default|GetExplosion)) 15.0 (Math|Random|RandomFloatinRange 1.5e+04 2.25e+04) false)
      (Transformation|SetWorldScale3D (Variables|Default|GetExplosion) (Math|Vector|MakeVector _returnvalue _returnvalue _returnvalue))
      (Transformation|SetWorldRotation (Variables|Default|GetFirelinger) "0,0.000000, 0" false false)
      (Components|Activation|Activate (Variables|Default|GetExplosion) false)
      (Utilities|FlowControl|Delay 0.5))
    (:then_3
      (Collision|SetActorEnableCollision false)
      (CallFunction|CleanUpComponents)
      (goto _label))))

(event Custom|Fuse
  (params (Controller :type Controller%20Object%20Reference) (Impulse :type Vector) (ImpactPoint :type Vector) (InteractedWith :type Boolean))
  (bind _explosionorigin (Variables|Default|GetExplosionOrigin))
  (bind _placeableinventory (Variables|Default|GetPlaceableInventory))
  (bind _returnvalue (Transformation|GetWorldLocation _explosionorigin))
  (bind _returnvalue_2 (Class|ItemInventory|GetResourceCount _placeableinventory 22120002 false))
  (bind _returnvalue_3 (Class|ItemInventory|GetResourceCount _placeableinventory 14183 false))
  (bind _returnvalue_4 (Class|ItemInventory|GetResourceCount _placeableinventory 22120004 false))
  (bind _returnvalue_5 (/ _returnvalue_2 6))
  (bind _returnvalue_6 (/ _returnvalue_4 2))
  (bind _returnvalue_7 (* _returnvalue_3 4))
  (bind _returnvalue_8 (+ _returnvalue_5 _returnvalue_7 _returnvalue_6))
  (bind _returnvalue_9 (Math|Conversions|ToFloat(Integer) _returnvalue_8))
  (bind _returnvalue_10 (* _returnvalue_8 9))
  (bind _returnvalue_11 (Math|Float|Power _returnvalue_9 0.333333333333))
  (bind _returnvalue_12 (* _returnvalue_11 4.5e+02))
  (bind _returnvalue_13 (* _returnvalue_12 2.0))
  (bind _returnvalue_14 (/ _returnvalue_13 4.0))
  (CallFunction|StartRolling ImpactPoint InteractedWith)
  (Utilities|FlowControl|Delay (Math|Random|RandomFloatinRange 1.0 2.0))
  (if (not (Variables|Default|GetHasBlownUp))
    (Class|PersistenceComponent|SetDirty (Variables|Default|GetConanBuildingPersistence) true 5.0)
    (CallFunction|CleanUpComponents)
    (Utilities|FlowControl|Delay (Math|Random|RandomFloatinRange 0.2 0.5))
    (Math|Integer|CompareInt _returnvalue_8 0
      (:>
        (bind _asconan_game_state (Utilities|Casting|CastToConanGameState (Game|GetGameState)))
        (if (or (Class|ConanGameState|IsPVPAllowed _asconan_game_state) (Utilities|IsValid (CallFunction|GetInstigatorOfPlacement)))
          ;[1 1 1] Do not damage Resource actors, otherwise explosion could cause a fracturation of their destructible meshes
          (if (Networking|IsDedicatedServer)
            (Utilities|Array|Clear (Variables|Default|GetIgnoreActors))
            (else
              (bind _outactors (Actor|GetAllActorsOfClass "/Game/Systems/Survival/Gathering/BP_ResourceActor.BP_ResourceActor_C"))
              (bind _output_get (Variables|Default|SetIgnoreActors _outactors))))
          (Utilities|Array|Add _output_get self)
          (|ApplyRadialDamagewithFalloffAsync (Math|Conversions|ToFloat(Integer) (/ _returnvalue_10 3)) 0.0 _returnvalue (/ _returnvalue_12 3.0) _returnvalue_12 3.0 "/Game/Systems/Progression/DmgTypeHealth_BP.DmgTypeHealth_BP_C" 0 self (CallFunction|GetInstigatorOfPlacement) "ECC_GameTraceChannel17"
            (:then
              (|ApplyRadialDamagewithFalloffAsync (Math|Conversions|ToFloat(Integer) _returnvalue_10) 1.0 _returnvalue _returnvalue_14 _returnvalue_13 3.0 "/Game/Systems/Progression/DmgTypeHealth_BP.DmgTypeHealth_BP_C" 0 self (CallFunction|GetInstigatorOfPlacement) "ECC_Visibility"
                (:then
                  (|ApplyRadialDamagewithFalloffAsync (Math|Conversions|ToFloat(Integer) (* _returnvalue_10 12)) 0.0 _returnvalue _returnvalue_14 _returnvalue_13 3.0 "/Game/Systems/Combat/Dmg_Explosive.Dmg_Explosive_C" 0 self (CallFunction|GetInstigatorOfPlacement) "ECC_Visibility"
                    (:then
                      _)))))))
        (bind _returnvalue_15 (Game|SpawnActorfromClass "/Game/Items/Explosives/BP_Oil_Fire_Large.BP_Oil_Fire_Large_C" (Transformation|GetWorldTransform (Variables|Default|GetExclusivePlacementSphere)) "AlwaysSpawn" self (Pawn|GetControlledPawn (CallFunction|GetInstigatorOfPlacement))))
        (Variables|/Game/Items/Weapons/Orbs/BP_Orb_Effect_Master.BP_Orb_Effect_Master_C|SetShouldBePlayerDamage _returnvalue_15 true)
        (CallFunction|MulticastExplosion)
        (Utilities|FlowControl|Delay 3e+01)
        (Actor|DestroyActor)
        (Class|GameEventDBLibrary|LogGameEventBuildableDemolished self 0 0 true)))))

(event Custom|StartRolling
  (params (ImpactPoint :type Vector) (InteractedWith :type Boolean))
  ;[1 1 1] Rolling
)

(event Custom|StopRolling
  ;[1 1 1] Rolling
)

(event EventBeginPlay
  (if (Class|CraftingQueue|IsRunning (Variables|Default|GetCraftingQueue))
    _
    (else
      (Default|TurnOffAll (Variables|Default|GetBP_BAC_TurnLightOnOff))))
  (|CallParentFunction)
  (Variables|Default|SetTimeCreated (Utilities|Time|GetGameTimeinSeconds))
  (if (Variables|Default|GetHasBlownUp)
    (Actor|DestroyActor)))

(event Game|Damage|EventAnyDamage
  (params (Damage :type Float%20%28single-precision%29) (DamageType :type Damage%20Type%20Object%20Reference) (InstigatedBy :type Controller%20Object%20Reference) (DamageCauser :type Actor%20Object%20Reference) (DamageEventID :type Integer))
  (bind _returnvalue (Math|Float|Truncate Damage))
  (bind _explosionorigin (Variables|Default|GetExplosionOrigin))
  (bind _placeableinventory (Variables|Default|GetPlaceableInventory))
  (bind _returnvalue_2 (Transformation|GetWorldLocation _explosionorigin))
  (bind _returnvalue_3 (Class|ItemInventory|GetResourceCount _placeableinventory 22120002 false))
  (bind _returnvalue_4 (Class|ItemInventory|GetResourceCount _placeableinventory 14183 false))
  (bind _returnvalue_5 (Class|ItemInventory|GetResourceCount _placeableinventory 22120004 false))
  (bind _returnvalue_6 (/ _returnvalue_3 6))
  (bind _returnvalue_7 (/ _returnvalue_5 2))
  (bind _returnvalue_8 (* _returnvalue_4 4))
  (bind _returnvalue_9 (+ _returnvalue_6 _returnvalue_8 _returnvalue_7))
  (bind _returnvalue_10 (Math|Conversions|ToFloat(Integer) _returnvalue_9))
  (bind _returnvalue_11 (* _returnvalue_9 9))
  (bind _returnvalue_12 (Math|Float|Power _returnvalue_10 0.333333333333))
  (bind _returnvalue_13 (* _returnvalue_12 4.5e+02))
  (bind _returnvalue_14 (* _returnvalue_13 2.0))
  (bind _returnvalue_15 (/ _returnvalue_14 4.0))
  ;[1 1 1] Bench Damaged
  (Development|PrintString (Utilities|String|Append (Utilities|String|ToString(Float) Damage) "Damage Detected on Alchemical Mixer, Truncated to " (Utilities|String|ToString(Integer) _returnvalue)))
  (Math|Integer|CompareInt 0 _returnvalue
    (:<
      (Development|PrintString "More than zero damage was done to the Mixer")
      (Math|Integer|CompareInt (Math|Random|RandomInteger 25) _returnvalue
        (:==
          _)
        (:<
          _))
      (Class|GameEventDBLibrary|LogGameEventBuildableDemolished self 0 (stale _asconan_character) false)
      (Development|PrintString "It was enough damage to randomly explode")
      (if (not (Variables|Default|GetIsABrush))
        (if (not (< (- (Utilities|Time|GetGameTimeinSeconds) (Variables|Default|GetTimeCreated)) 1.0)) ; If  the jar has just been placed, don't explode it yet, just start the fuse
          (if (not (Variables|Default|GetHasBlownUp))
            (Class|PersistenceComponent|SetDirty (Variables|Default|GetConanBuildingPersistence) true 5.0)
            (CallFunction|CleanUpComponents)
            (Utilities|FlowControl|Delay (Math|Random|RandomFloatinRange 0.2 0.5))
            (Math|Integer|CompareInt _returnvalue_9 0
              (:>
                (bind _asconan_game_state (Utilities|Casting|CastToConanGameState (Game|GetGameState)))
                (if (or (Class|ConanGameState|IsPVPAllowed _asconan_game_state) (Utilities|IsValid (CallFunction|GetInstigatorOfPlacement)))
                  ;[1 1 1] Do not damage Resource actors, otherwise explosion could cause a fracturation of their destructible meshes
                  (if (Networking|IsDedicatedServer)
                    (Utilities|Array|Clear (Variables|Default|GetIgnoreActors))
                    (else
                      (bind _outactors (Actor|GetAllActorsOfClass "/Game/Systems/Survival/Gathering/BP_ResourceActor.BP_ResourceActor_C"))
                      (bind _output_get (Variables|Default|SetIgnoreActors _outactors))))
                  (Utilities|Array|Add _output_get self)
                  (|ApplyRadialDamagewithFalloffAsync (Math|Conversions|ToFloat(Integer) (/ _returnvalue_11 3)) 0.0 _returnvalue_2 (/ _returnvalue_13 3.0) _returnvalue_13 3.0 "/Game/Systems/Progression/DmgTypeHealth_BP.DmgTypeHealth_BP_C" 0 self (CallFunction|GetInstigatorOfPlacement) "ECC_GameTraceChannel17"
                    (:then
                      (|ApplyRadialDamagewithFalloffAsync (Math|Conversions|ToFloat(Integer) _returnvalue_11) 1.0 _returnvalue_2 _returnvalue_15 _returnvalue_14 3.0 "/Game/Systems/Progression/DmgTypeHealth_BP.DmgTypeHealth_BP_C" 0 self (CallFunction|GetInstigatorOfPlacement) "ECC_Visibility"
                        (:then
                          (|ApplyRadialDamagewithFalloffAsync (Math|Conversions|ToFloat(Integer) (* _returnvalue_11 12)) 0.0 _returnvalue_2 _returnvalue_15 _returnvalue_14 3.0 "/Game/Systems/Combat/Dmg_Explosive.Dmg_Explosive_C" 0 self (CallFunction|GetInstigatorOfPlacement) "ECC_Visibility"
                            (:then
                              _)))))))
                (bind _returnvalue_16 (Game|SpawnActorfromClass "/Game/Items/Explosives/BP_Oil_Fire_Large.BP_Oil_Fire_Large_C" (Transformation|GetWorldTransform (Variables|Default|GetExclusivePlacementSphere)) "AlwaysSpawn" self (Pawn|GetControlledPawn (CallFunction|GetInstigatorOfPlacement))))
                (Variables|/Game/Items/Weapons/Orbs/BP_Orb_Effect_Master.BP_Orb_Effect_Master_C|SetShouldBePlayerDamage _returnvalue_16 true)
                (CallFunction|MulticastExplosion)
                (Utilities|FlowControl|Delay 3e+01)
                (Actor|DestroyActor)
                (Class|GameEventDBLibrary|LogGameEventBuildableDemolished self 0 0 true)))))))))

(event Collision|EventActorBeginOverlap
  (params (OtherActor :type Actor%20Object%20Reference)))

(fn ConstructionScript
  (|CallParentFunction))

(fn GetArtisanThrallInventory
  (return (Variables|Default|GetThrallInventory)))

(fn IsPlayerDamage
  ;[1 1 1] Explosive jars are always player damage
  (return true))

(fn IsThrallDamage
  (return false))

(fn GetAttackerUniqueID
  (return (Variables|Default|GetOwnerUniqueID)))

(fn CanStationUseThralls
  (|CallParentFunction)
  (return true))