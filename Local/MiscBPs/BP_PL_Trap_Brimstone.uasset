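; Brimstone trap Blueprint that explodes and leaves a growing, timed gas hazard.
; DealDamage runs the parent logic, then spawns a BP_GrowingHazardArea at the gas particle point that applies a gas buff with a corpse-rot cloud.
; Outside dedicated servers, activation stops fuse effects and, only if the dud smoke is valid, plays explosion effects and camera shake and hides the mesh.
; Placement checks and construction defer to the parent.
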(event `self.Deal_Damage`
  (`parent.Deal_Damage`)
  (`|SpawnActorFromClass` "/Game/Environment/Hazards/BP_GrowingHazardArea.BP_GrowingHazardArea_C" (`KismetMathLibrary.MakeTransform` (`SceneComponent.K2_GetComponentLocation` (`self.GasParticlePoint`)) (struct)) "AlwaysSpawn" "OverrideRootScale" null 750.0 "/Game/Systems/Buffs/Damage_Percent/00_BP_AC_Buff_Gas.00_BP_AC_Buff_Gas_C" 12.0 "/Game/Systems/Building/Placeables/Trebuchet/Trebuchet_V2/Particles/P_CorpseRotCloud.P_CorpseRotCloud"))

(event `self.Play Trap Activate Effects`
  (bind _staticmesh (`self.StaticMesh`))
  (bind _returnvalue (`SceneComponent.K2_GetComponentLocation` _staticmesh))
  ;[1 0.6413 0.1882] Effects
  (if (not (`KismetSystemLibrary.IsDedicatedServer`))
    ;;[0.02499 0.09524 0.16] Disable dud effects.
    (bind _fusesound (`self.FuseSound`)
      (:`then`
        (`ConanAudioComponent.Stop` _fusesound))
      (:`else`
        _))
    (bind _fusedudsmoke (`self.FuseDudSmoke`)
      (:`then`
        (`ActorComponent.Deactivate` _fusedudsmoke)
        (`GameplayStatics.PlaySoundAtLocation` (`self.S_Trigger_Activate`) _returnvalue)
        (`ActorComponent.Activate` (`self.Explosion`) false)
        (`GameplayStatics.PlayWorldCameraShake` "/Game/Items/Explosives/CameraShake_Explosion_Small.CameraShake_Explosion_Small_C" _returnvalue 0.0 3200.0 1.0 true)
        (`SceneComponent.SetVisibility` _staticmesh false false))
      (:`else`))))

(fn `CanBePlaced`
  (params (AttachTo :type "BuildableBase Object Reference") (InstanceIndex :type Integer))
  (returns (FailedMessage :type String) (ReturnValue :type "ECanBePlacedResult Enum"))
  (bind (_failedmessage _returnvalue) (`parent.CanBePlaced` AttachTo InstanceIndex))
  (return _failedmessage _returnvalue))

(fn `UserConstructionScript`
  (`parent.UserConstructionScript`))