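; Player battering ram item that puts its wielder in a carry substate, re-entered after each attack.
; Equipping sets the building damage multiplier stat and binds to the controller's instigated-damage event; unequipping exits the substate and unbinds.
; Non-explosive health damage against characters triggers extra knockback damage.
; A cooldown-gated radial explosive hit on buildables, ignoring the owner and their floor, exists but is disconnected.
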(event `self.OnEquip`
  (params (owner :type "Character Object Reference"))
  (`parent.OnEquip` owner)
  (bind _asconan_character (`self.CarryTime` owner))
  (`ConanCharacter.SetFloatStat` _asconan_character "BuildingDamageMultiplier" 2.0)
  (add `Controller.OnInstigatedAnyDamage` (`ConanCharacter.GetOwningController` _asconan_character) (delegate `SiegeDamageProc`)))

(event `SiegeDamageProc`
  (params (Damage :type "Float (double-precision)") (DamageType :type "DamageType Object Reference") (DamagedActor :type "Actor Object Reference") (DamageCauser :type "Actor Object Reference"))
  (bind _returnvalue (`GameplayStatics.GetObjectClass` DamageType))
  (if (and (`KismetMathLibrary.ClassIsChildOf` _returnvalue "/Game/Systems/Progression/DmgTypeHealth_BP.DmgTypeHealth_BP_C") (not (`KismetMathLibrary.ClassIsChildOf` _returnvalue "/Game/Systems/Combat/Dmg_Explosive.Dmg_Explosive_C")))
    (`|ExecutionSequence`
      (:`then_1`
        (bind _asconan_character (cast `ConanCharacter` DamagedActor))
        (`GameplayStatics.ApplyDamage` _asconan_character 2.0 null (`self.VisualActor`) "/Game/Systems/Combat/DamageTypes/BP_Knockback_NPC_Away_Back.BP_Knockback_NPC_Away_Back_C") ; KNOCKBACK!
      ))))

(event `self.EndAttacking`
  (`parent.EndAttacking`)
  (`self.CarryTime` (stale `self.OnEquip` owner)))

(event `self.OnUnEquip`
  (params (owner :type "Character Object Reference"))
  (`parent.OnUnEquip` owner)
  (message `/Game/Systems/Interfaces/BaseBPCharInterface.ExitSubstateInterface` owner "NewEnumerator33")
  (bind _asconan_character (cast `ConanCharacter` owner))
  (remove `Controller.OnInstigatedAnyDamage` (`ConanCharacter.GetOwningController` _asconan_character) (`|CreateDelegate` :!event `SiegeDamageProc`)))

(fn `CanDoSiegeProc`
  (returns (CanDo :type Boolean))
  (bind _asconan_game_state (cast `ConanGameState` (`GameplayStatics.GetGameState`))
    (:`then`
      (return (> (- (`ConanGameState.GetBPServerRuntime` _asconan_game_state) 1.0) (`self.LastSiegeHit`))))
    (:`CastFailed`
      (return false))))

(fn `FindOwnerFloor`
  (returns (Floor :type "Actor Object Reference"))
  (bind _asconan_character (cast `ConanCharacter` (`self.GetOwner`))
    (:`then`
      (bind (_bblockinghit _bwalkablefloor _blinetrace _floordist _linedist _hitresult) (break `FindFloorResult` (`CharacterMovementComponent.CurrentFloor` (`Character.CharacterMovement` _asconan_character))))
      (if _bwalkablefloor
        (return (`.HitActor` (`GameplayStatics.BreakHitResult` _hitresult)))
        (else
          (return null))))
    (:`CastFailed`
      (return null))))

(fn `SetSiegeCooldown`
  (bind _asconan_game_state (cast `ConanGameState` (`GameplayStatics.GetGameState`)))
  (set `self.LastSiegeHit` (`ConanGameState.GetBPServerRuntime` _asconan_game_state)))