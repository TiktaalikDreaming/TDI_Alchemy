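; BP_CustomArrow_GlowArea_TDI is a glow-area actor whose point light dims in steps until the actor destroys itself.
; BeginPlay sets a looping 30-second timer that starts a new looping 12-second fade timer each time it fires.
; Each fade tick lowers the light intensity by a fixed amount, destroying the actor once it drops below zero.
; The construction script collapses the TriggerSphere radius to zero.
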(event `self.ReceiveBeginPlay`
  (bind _returnvalue (`KismetSystemLibrary.K2_SetTimerDelegate` (delegate `Start Timer`) 30.0 true))
  (set `self.StartFade` _returnvalue))

(event `Start Timer`
  (bind _returnvalue (`KismetSystemLibrary.K2_SetTimerDelegate` (delegate `LightsOnUpdate`) 12.0 true))
  (set `self.FadeTimer` _returnvalue))

(event `LightsOnUpdate`
  (`self.FadeOut`))

(fn `FadeOut`
  (bind _output_get (set `self.Intensity` (- (`self.Intensity`) 100.0)))
  (`LightComponent.SetIntensity` (`self.PointLight`) _output_get)
  (if (< (`self.Intensity`) 0.0)
    (`self.K2_DestroyActor`)))

(fn `UserConstructionScript`
  (bind _trigger_sphere (`self.Trigger Sphere`))
  (if (!= (`SphereComponent.SphereRadius` _trigger_sphere) 0.0)
    (`SphereComponent.SetSphereRadius` _trigger_sphere 0.0 true)))