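; Stackable Slowed buff that snares its owner by lowering movement speed through the combat interface.
; For non-NPC owners the snare scales with stack size, and the resulting multiplier is clamped to a floor before being applied.
; Buff start and client-side stack changes share that path, with IsServer checks avoiding double application, while clearing restores full speed.
; A perk-based cripple modifier branch is disconnected.
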(event `self.InitBuff`
  (params (OwningCharacter :type "ConanCharacter Object Reference") (Instigator :type "Controller Object Reference"))
  (`parent.InitBuff` OwningCharacter Instigator)
  (bind _asis_base_bpcombat_interface (cast `/Game/Systems/Interfaces/IsBaseBPCombatInterface` (`self.OwningCharacter`)))
  (set `self.CombatInterface` _asis_base_bpcombat_interface))

(event `self.AdjustStackSize`
  (params (StackAdjustment :type Integer))
  (bind _returnvalue (* (`self.StackSize`) (`self.SnareValuePlayer`)))
  (`parent.AdjustStackSize` StackAdjustment)
  (if (not (`KismetSystemLibrary.IsServer`))
    (bind _isnpc (message `/Game/Systems/Interfaces/BaseBPCharInterface.CheckIsNPC` (`self.OwningCharacter`) :!label _label))
    (if (not _isnpc)
      (set `self.SnareValue` _returnvalue)
      (`KismetSystemLibrary.PrintString` (`KismetStringLibrary.Conv_DoubleToString` _returnvalue)))
    (bind _output_get (set `self.MovementSpeedMultiplier` (`KismetMathLibrary.FClamp` (- 1.0 (`self.SnareValue`)) 0.05)))
    (`KismetSystemLibrary.PrintString` (`KismetStringLibrary.Conv_DoubleToString` _output_get))
    (`/Game/Systems/Interfaces/IsBaseBPCombatInterface.AdjustMovementSpeedMultiplier` (`self.CombatInterface`) true _output_get)))

(event `self.GameplayEffectToApplyOnBuffStart`
  (`parent.GameplayEffectToApplyOnBuffStart`)
  (goto _label))

(event `self.ClientStartBuff`
  (params (OwningCharacter :type "ConanCharacter Object Reference") (Duration :type "Float (single-precision)"))
  (`parent.ClientStartBuff` OwningCharacter Duration)
  (bind _asis_base_bpcombat_interface (cast `/Game/Systems/Interfaces/IsBaseBPCombatInterface` (`self.OwningCharacter`)))
  (set `self.CombatInterface` _asis_base_bpcombat_interface)
  ;[1 1 1] If we didn’t do this; then it would apply the effect twice
  (if (not (`KismetSystemLibrary.IsServer`))
    (goto _label)))

(event `self.GameplayEffectToApplyOnBuffCleared`
  (`parent.GameplayEffectToApplyOnBuffCleared`)
  (bind _output_get (set `self.MovementSpeedMultiplier` 1.0 :!label _label_2))
  (`/Game/Systems/Interfaces/IsBaseBPCombatInterface.AdjustMovementSpeedMultiplier` (`self.CombatInterface`) true _output_get))

(event `self.ClientClearBuff`
  (params (OwningCharacter :type "ConanCharacter Object Reference"))
  (`parent.ClientClearBuff` OwningCharacter)
  ;[1 1 1] If we didn’t do this; then it would apply the effect twice
  (if (`KismetSystemLibrary.IsServer`)
    (goto _label_2)
    (else
      (goto _label_2))))

(fn `GetCurrentStack`
  (returns (ReturnValue :type Integer))
  (return (`parent.GetCurrentStack`)))

(fn `GetEffectDescription`
  (returns (Description :type Text))
  (return (`|FormatText` "Movement Speed reduced  by {SpeedModifier}%" (`KismetMathLibrary.Round` (* (- 1.0 (`self.MovementSpeedMultiplier`)) 100.0)))))